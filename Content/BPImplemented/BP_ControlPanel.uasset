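; Elevator control panel that builds a grid of tagged, numbered floor buttons at runtime, one per floor.
; BeginPlay loops over the floor count, adding static mesh buttons from the template button's transform and wrapping to a new row at the horizontal limit.
; Each button gets an ElevatorButton tag plus a zero-based floor index tag, and a one-based text label.
; The same loop tells the referenced elevator's call button to spawn a button for each index.
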(event EventBeginPlay
  (Variables|ConrtolPanelButtons|SetControl%20Panel%20Button%20Offset%20Cache (Variables|ConrtolPanelButtons|GetControlPanelButtonOffset))
  (Variables|Default|SetMax%20Horizontal%20Buttons%20Cache (Variables|ConrtolPanelButtons|GetMaxHorizontalButtons))
  (Variables|Default|SetStartTransform (Transformation|GetRelativeTransform (Variables|Default|GetPanelButton)))
  (for _index (range 1 (Variables|ElevatorSystem|GetNumberOfFloors))
    (Variables|Default|SetCurrent%20Line%20Value _index)
    (if (> (Variables|Default|GetCurrent%20Line%20Value) (Variables|ConrtolPanelButtons|GetMaxHorizontalButtons))
      (Variables|Default|SetNewLineValue (+ (Variables|Default|GetNewLineValue) (Variables|Default|GetCPDistanceBetVer)))
      (Variables|ConrtolPanelButtons|SetControlPanelButtonOffset (Variables|ConrtolPanelButtons|GetControl%20Panel%20Button%20Offset%20Cache))
      (Variables|ConrtolPanelButtons|SetMaxHorizontalButtons (+ (Variables|ConrtolPanelButtons|GetMaxHorizontalButtons) (Variables|Default|GetMax%20Horizontal%20Buttons%20Cache))))
    (bind _returnvalue (AddComponent|AddStaticMeshComponent false (Variables|Default|GetStartTransform)))
    (bind _output_get (Variables|Default|SetButtonMeshCompRef _returnvalue))
    (Variables|/Script/Engine.ActorComponent|SetComponentTags _output_get (Utilities|Array|MakeArray "ElevatorButton" (Utilities|String|StringToName (Utilities|String|ToString(Integer) (- (Variables|Default|GetCurrent%20Line%20Value) 1)))))
    (Transformation|SetRelativeLocation (Variables|Default|GetButtonMeshCompRef) (Math|Vector|MakeVector (.x (.location (Variables|Default|GetStartTransform))) (- (Variables|ConrtolPanelButtons|GetControlPanelButtonOffset) (.y (.location (Variables|Default|GetStartTransform)))) (- (.z (.location (Variables|Default|GetStartTransform))) (Variables|Default|GetNewLineValue))) false false)
    (Variables|ConrtolPanelButtons|SetControlPanelButtonOffset (- (Variables|ConrtolPanelButtons|GetControlPanelButtonOffset) (Variables|Default|GetCPDistanceBetHor)))
    (Default|SpawnButton (Variables|/Game/BPImplemented/BP_Lift.BP_Lift_C|GetElevatorCallButton (Variables|ElevatorSystem|GetElevatorRef)) (Utilities|String|StringToName (Utilities|String|ToString(Integer) (- (Variables|Default|GetCurrent%20Line%20Value) 1))))
    (bind _returnvalue_2 (AddComponent|AddTextRenderComponent false (Math|Transform|MakeTransform (Math|Vector|MakeVector (.x (Variables|/Script/Engine.SceneComponent|GetRelativeLocation (Variables|Default|GetButtonMeshCompRef))) (.y (Variables|/Script/Engine.SceneComponent|GetRelativeLocation (Variables|Default|GetButtonMeshCompRef))) (.z (Variables|/Script/Engine.SceneComponent|GetRelativeLocation (Variables|Default|GetButtonMeshCompRef)))) "0, 0, 0" "1.000000,1.000000,1.000000")))
    (Rendering|Components|TextRender|SetText _returnvalue_2 (Utilities|Text|ToText(Integer) (+ (Math|Conversions|ToInteger(Byte) (Utilities|String|ToString(Text) (Utilities|Text|ToText(Name) (Utilities|String|StringToName (Utilities|String|ToString(Integer) (- (Variables|Default|GetCurrent%20Line%20Value) 1)))))) 1)))))

(fn ConstructionScript)