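; BP_Button is an elevator button actor that shows a widget while something overlaps its Trigger.
; SpawnButton adds a call-button static mesh component based on the Button's transform, with depth and horizontal offsets.
; It tags the call button with "ElevatorCallButton" and the floor value, then increments CallButtonHeight by the elevator's floor height.
; The vertical offset calculation is left unconnected.
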(event OnComponentBeginOverlap(Trigger)
  (params (OverlappedComponent :type Primitive%20Component%20Object%20Reference) (OtherActor :type Actor%20Object%20Reference) (OtherComp :type Primitive%20Component%20Object%20Reference) (OtherBodyIndex :type Integer) (bFromSweep :type Boolean) (SweepResult :type Hit%20Result%20Structure%20%28by%20ref%29))
  ;[0.3438 0.2997 0.1385] Widget Visibility
  (Rendering|SetVisibility (Variables|Default|GetWidget) true false))

(event OnComponentEndOverlap(Trigger)
  (params (OverlappedComponent :type Primitive%20Component%20Object%20Reference) (OtherActor :type Actor%20Object%20Reference) (OtherComp :type Primitive%20Component%20Object%20Reference) (OtherBodyIndex :type Integer))
  ;[0.3438 0.2997 0.1385] Widget Visibility
  (Rendering|SetVisibility (Variables|Default|GetWidget) false false))

(event Custom|SpawnButton
  (params (FloorValue :type Name))
  (bind _button (Variables|Default|GetButton))
  (bind _returnvalue (Transformation|GetRelativeTransform _button))
  (bind _location (Math|Transform|BreakTransform _returnvalue))
  (bind (_x _y _z) (Math|Vector|BreakVector _location))
  (Variables|Default|SetFloor%20Value FloorValue)
  (bind _returnvalue_2 (AddComponent|AddStaticMeshComponent false (Transformation|GetRelativeTransform (Variables|Default|GetButton))))
  (Components|StaticMesh|SetStaticMesh _returnvalue_2 (Variables|Default|GetCallButtonMesh))
  (Variables|Default|SetCallButtonRef 0)
  (Transformation|SetRelativeLocation (Variables|Default|GetCallButtonRef) (Math|Vector|MakeVector (- _x (Variables|Default|GetCallButtonDepthOffset)) (- _y (Variables|Default|GetCallButtonHorOffset)) 0.0) false false)
  (Variables|/Script/Engine.ActorComponent|SetComponentTags (Variables|Default|GetCallButtonRef) (Utilities|Array|MakeArray "ElevatorCallButton" (Variables|Default|GetFloor%20Value)))
  (Variables|Default|SetCallButtonHeight (+ (Variables|Default|GetCallButtonHeight) (Variables|/Game/BPImplemented/BP_Lift.BP_Lift_C|GetHeightOfFloor (Variables|Default|GetElevatorRef)))))

(fn ConstructionScript)